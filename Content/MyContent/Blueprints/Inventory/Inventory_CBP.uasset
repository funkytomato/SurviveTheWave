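; Inventory Blueprint that stores the item list and toggles the inventory screen.
; InventoryEvent uses a FlipFlop to pause the game, show InventorySystemContainer_WBP with the mouse cursor and remove PlayerHUD_WBP, then reverse this, creating a fresh HUD.
; AddItemToInventory simply appends to the Inventory array, as its quantity-stacking logic is disconnected.
; RetrieveItem searches linearly by item name, printing a message when none matches.
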(event `InventoryEvent`
  (bind _returnvalue (`GameplayStatics.GetPlayerController` 0))
  (`/Engine/EditorBlueprintResources/StandardMacros.FlipFlop`
    (:`A`
      (`GameplayStatics.SetGamePaused` (`self.Paused`))
      (bind _returnvalue_2 (`|CreateWidget` "/Game/MyContent/Blueprints/Inventory/InventorySystemContainer_WBP.InventorySystemContainer_WBP_C" (`GameplayStatics.GetPlayerController` 0)))
      (`UserWidget.AddToViewport` _returnvalue_2 0)
      (set `PlayerController.bShowMouseCursor` true _returnvalue)
      (bind _foundwidgets (`WidgetBlueprintLibrary.GetAllWidgetsOfClass` "/Game/MyContent/UI/PlayerHUD_WBP.PlayerHUD_WBP_C"))
      (`Widget.RemoveFromParent` _foundwidgets))
    (:`B`
      (`GameplayStatics.SetGamePaused` (`self.UnPaused`))
      (`Widget.RemoveFromParent` _returnvalue_2)
      (set `PlayerController.bShowMouseCursor` false _returnvalue)
      (bind _returnvalue_3 (`|CreateWidget` "/Game/MyContent/UI/PlayerHUD_WBP.PlayerHUD_WBP_C" (`GameplayStatics.GetPlayerController` 0)))
      (`UserWidget.AddToViewport` _returnvalue_3 0))))

(fn `AddItemToInventory`
  (params (itemToAdd :type "/Game/MyContent/Blueprints/Inventory/InventoryItemStruct Structure"))
  (locals (itemChanged :type "/Game/MyContent/Blueprints/Inventory/InventoryItemStruct Structure"))
  (`KismetSystemLibrary.PrintString` (`KismetStringLibrary.Conv_IntToString` (`KismetArrayLibrary.Array_Length` (`self.Inventory`))))
  (`KismetArrayLibrary.Array_Add` (`self.Inventory`) itemToAdd))

(fn `RetrieveItem`
  (params (itemToFind :type "/Game/MyContent/Blueprints/Inventory/InventoryItemType Enum" :default "NewEnumerator0"))
  (returns (itemFound :type "/Game/MyContent/Blueprints/Inventory/InventoryItemStruct Structure"))
  (locals (name :type "/Game/MyContent/Blueprints/Inventory/InventoryItemType Enum"))
  (set `local.name` itemToFind)
  (for _array_element (`self.Inventory`)
    (if (`|EnumEquality` (`.ItemName_10_CE6047ECE142A1033D009FBB173057C7` (break `/Game/MyContent/Blueprints/Inventory/InventoryItemStruct` _array_element)) (`local.name`))
      (return _array_element)))
  (`KismetSystemLibrary.PrintString` "Item not found")
  (`KismetSystemLibrary.PrintString` (`|GetEnumeratorNameAsString` (`local.name`)))
  (return))