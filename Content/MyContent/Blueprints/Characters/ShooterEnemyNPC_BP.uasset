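; Enemy shooter NPC, a child Blueprint that configures the rifle it carries and inherits the rest from its parent.
; The construction script stores the Gun child actor as the equipped BFX_Rifle_BP, snaps it to the mesh's right weapon socket and takes ownership.
; Weapon Setup extends the parent's, switching on AI weapon type to fire the rifle's matching select event.
; The Sniper Rifle type calls the pistol select event.
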(event `self.ReceiveBeginPlay`
  (`parent.ReceiveBeginPlay`))

(fn `UserConstructionScript`
  (`parent.UserConstructionScript`)
  (bind _asbfx_rifle_bp (cast `/Game/MyContent/Blueprints/Characters/BFX_Rifle_BP` (`ChildActorComponent.ChildActor` (`self.Gun`))))
  (set `self.EquippedGun` _asbfx_rifle_bp)
  (`SceneComponent.K2_AttachToComponent` (`self.Gun`) (`self.Mesh`) "weapon_rSocket" "SnapToTarget" "SnapToTarget" "SnapToTarget" true)
  (`self.SetOwner` (`self.EquippedGun`) self))

(fn `Weapon Setup`
  (`parent.Weapon Setup`)
  (switch `/Game/ShooterSimplifiedAI/Blueprints/AI/E_AI_WeaponType` (`self.AIWeponTypes`)
    (:`NewEnumerator0`
      (bind _asbfx_rifle_bp (cast `/Game/MyContent/Blueprints/Characters/BFX_Rifle_BP` (`ChildActorComponent.ChildActor` (`self.Gun`))))
      (`/Game/MyContent/Blueprints/Characters/BFX_Rifle_BP.RifleSelectEvent` _asbfx_rifle_bp))
    (:`NewEnumerator1`
      (bind _asbfx_rifle_bp_2 (cast `/Game/MyContent/Blueprints/Characters/BFX_Rifle_BP` (`ChildActorComponent.ChildActor` (`self.Gun`))))
      (`/Game/MyContent/Blueprints/Characters/BFX_Rifle_BP.SelectHPRifleEvent` _asbfx_rifle_bp_2))
    (:`NewEnumerator2`
      (bind _asbfx_rifle_bp_3 (cast `/Game/MyContent/Blueprints/Characters/BFX_Rifle_BP` (`ChildActorComponent.ChildActor` (`self.Gun`))))
      (`/Game/MyContent/Blueprints/Characters/BFX_Rifle_BP.PistolSelectEvent` _asbfx_rifle_bp_3))))