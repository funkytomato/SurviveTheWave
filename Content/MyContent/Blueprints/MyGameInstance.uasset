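; Game instance that keeps the elapsed game time as minutes and seconds.
; StartGame resets both counters and starts a looping one-second timer that calls LevelTimer, which counts seconds and rolls them over into minutes.
; PauseGame and UnpauseGame pause and resume that timer through its stored handle.
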(event `StartGame`
  (`self.InitialiseGameVariables`)
  (bind _returnvalue (`KismetSystemLibrary.K2_SetTimer` null "LevelTimer" 1.0 true))
  (set `self.LevelTimerRef` _returnvalue))

(event `PauseGame`
  (`KismetSystemLibrary.K2_PauseTimerHandle` (`self.LevelTimerRef`)))

(event `UnpauseGame`
  (`KismetSystemLibrary.K2_UnPauseTimerHandle` (`self.LevelTimerRef`)))

(event `InitialiseGameVariables`
  ;[1 1 1] Initialise Time Properties
  (set `self.Seconds` 0)
  (set `self.Minutes` 0))

(fn `LevelTimer`
  (set `self.Seconds` (+ (`self.Seconds`) 1))
  (if (> (`self.Seconds`) 59)
    (set `self.Minutes` (+ (`self.Minutes`) 1))
    (set `self.Seconds` 0)))