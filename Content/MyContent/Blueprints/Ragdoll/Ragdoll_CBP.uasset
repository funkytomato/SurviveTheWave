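; Ragdoll component that gives a character partial-body physical hit reactions, with unconnected setup code targeting ShooterEnemyNPC_BP.
; HitReaction simulates bodies below the pelvis bone, applies HitReactionProfile and adds an impulse along the shot direction, redirecting pelvis hits to spine_01.
; TogglePhysicalAnimation flips that simulation on, half blended, and off.
; BeginPlay and Tick are empty; the component setup and timed blend-out logic exist but never run.
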(event `self.ReceiveBeginPlay`)

(event `TogglePhysicalAnimation`
  (bind _physicalanimcomp (`self.PhysicalAnimComp`))
  (`/Engine/EditorBlueprintResources/StandardMacros.FlipFlop`
    (:`A`
      (`Actor.SetActorEnableCollision` (`self.MyCharacter`) true)
      (`SkeletalMeshComponent.SetAllBodiesBelowSimulatePhysics` (`self.Mesh`) "Pelvis" true false)
      (`PhysicalAnimationComponent.ApplyPhysicalAnimationProfileBelow` _physicalanimcomp "Pelvis" "HitReactionProfile" false false)
      (`PhysicalAnimationComponent.SetStrengthMultiplyer` _physicalanimcomp 0.0)
      (`SkeletalMeshComponent.SetAllBodiesBelowPhysicsBlendWeight` (`self.Mesh`) "Pelvis" 0.5 false true))
    (:`B`
      (`SkeletalMeshComponent.SetAllBodiesBelowSimulatePhysics` (`self.Mesh`) "Pelvis" false false))))

(event `HitReaction`
  (params (Hit :type "HitResult Structure"))
  (bind (_bblockinghit _binitialoverlap _time _distance _location _impactpoint _normal _impactnormal _physmat _hitactor _hitcomponent _hitbonename _hititem _elementindex _faceindex _tracestart _traceend) (`GameplayStatics.BreakHitResult` Hit))
  (`self.SetComponentTickEnabled` true)
  (set `self.HitReactionTimeRemaining` (+ (`self.HitReactionTimeRemaining`) 2.0))
  (`PhysicalAnimationComponent.ApplyPhysicalAnimationProfileBelow` (`self.PhysicalAnimComp`) "pelvis" "HitReactionProfile" false false)
  (`SkeletalMeshComponent.SetAllBodiesBelowSimulatePhysics` (`self.Mesh`) "Pelvis" true false)
  (`PrimitiveComponent.AddImpulse` (`self.Mesh`) (* (`KismetMathLibrary.Normal` (- _traceend _tracestart)) 500.0) (select `bool` (== _hitbonename "pelvis") :`false` _hitbonename :`true` "spine_01") true))

(event `self.ReceiveTick`
  (params (DeltaSeconds :type "Float (single-precision)")))