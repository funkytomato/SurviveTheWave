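; Health component that tracks an actor's health, armour and death state, reacting to bound damage and boost dispatchers.
; Headshot damage types multiply damage and bypass armour; other damage drains armour, applying full damage to health whenever armour is zero afterwards.
; Health changes broadcast UpdateHealth for the blood screen, and health damage on non-players spawns a damage popup widget at the owner's screen position.
; The armour boost handler is empty.
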(event `self.ReceiveBeginPlay`
  ;[1 1 1] Recieved Damage Event Dispatcher
  (add `self.RecieveDamage` (delegate `RecieveDamage_Event`))
  ;[1 1 1] Increase Boost Event Dispatcher
  (add `self.HealthBoost` (delegate `HealthBoost_Event`))
  (add `self.ArmorBoost` (delegate `ArmorBoost_Event`)))

(event `HealthBoost_Event` :!signature `self.HealthBoost`
  (params (healthBoost :type "Float (double-precision)"))
  ;[1 1 1] Increase Boost Event Dispatcher
  ;;[1 1 1] Increase Health
  (bind _currenthealth (`self.IncreaseHealth` healthBoost))
  ;;[1 1 1] Update Blood Screen
  (`self.UpdateHealth` _currenthealth))

(event `ArmorBoost_Event` :!signature `self.ArmorBoost`
  (params (boostAmount :type "Float (double-precision)")))

(event `RecieveDamage_Event` :!signature `self.RecieveDamage`
  (params (Damage :type "Float (double-precision)") (DamageType :type "DamageType Object Reference") (InstigatedBy :type "Controller Object Reference") (DamageCauser :type "Actor Object Reference"))
  (bind _asdamage_type_headshot (cast `/Game/MyContent/Blueprints/Health/DamageTypeHeadshot` DamageType)
    (:`then`
      (bind _returnvalue (* (`/Game/MyContent/Blueprints/Health/DamageTypeHeadshot.multiplier` _asdamage_type_headshot) Damage))
      ;[1 1 1] Apply Headshot increased Damage.  Show bloodscreen!!!!
      (bind _currenthealth (`self.DecreaseHealth` _returnvalue))
      (`self.UpdateHealth` _currenthealth)
      ;[1 1 1] Only Display Damage Recieved Widget if not Player
      (if (not (`self.IsPlayer?`))
        ;;[1 1 1] Display Damage Popup Widget
        (bind _returnvalue_2 (`|CreateWidget` "/Game/MyContent/UI/DamageRecieved_WBP.DamageRecieved_WBP_C" null false _returnvalue))
        (`UserWidget.AddToViewport` _returnvalue_2 0)
        (`UserWidget.SetPositionInViewport` _returnvalue_2 (`GameplayStatics.ProjectWorldToScreen` (`GameplayStatics.GetPlayerController` 0) (`Actor.K2_GetActorLocation` (`self.MyOwner`))) true)))
    (:`CastFailed`
      ;[1 1 1] Apply default damage and reduce armour before health.  Show bloodscreen!!!!
      (`self.DecreaseArmour` Damage)
      (if (`self.noArmour?`)
        (bind _currenthealth_2 (`self.DecreaseHealth` Damage))
        (`self.UpdateHealth` _currenthealth_2)
        (if (not (`self.IsPlayer?`))
          (bind _returnvalue_3 (`|CreateWidget` "/Game/MyContent/UI/DamageRecieved_WBP.DamageRecieved_WBP_C" null false Damage))
          (`UserWidget.AddToViewport` _returnvalue_3 0)
          (`UserWidget.SetPositionInViewport` _returnvalue_3 (`GameplayStatics.ProjectWorldToScreen` (`GameplayStatics.GetPlayerController` 0) (`Actor.K2_GetActorLocation` (`self.MyOwner`))) true))))))

(fn `DecreaseArmour`
  (params (amount :type "Float (double-precision)"))
  (bind _output_get (set `self.Armour` (`KismetMathLibrary.FClamp` (- (`self.Armour`) amount) 0.0 (`self.MaxArmour`))))
  (set `self.noArmour?` (== _output_get 0.0)))

(fn `DecreaseHealth`
  (params (value :type "Float (double-precision)"))
  (returns (currentHealth :type "Float (double-precision)"))
  (bind _output_get (set `self.Health` (`KismetMathLibrary.FClamp` (- (`self.Health`) value) 0.0 (`self.MaxHealth`))))
  (set `self.IsDead?` (not (> _output_get 0.0)))
  (return _output_get))

(fn `IncreaseArmour`
  (params (amount :type "Float (double-precision)"))
  (bind _output_get (set `self.Armour` (`KismetMathLibrary.FClamp` (+ (`self.Armour`) amount) 0.0 (`self.MaxArmour`))))
  (set `self.noArmour?` (not (> _output_get 0.0))))

(fn `IncreaseHealth`
  (params (value :type "Float (double-precision)"))
  (returns (currentHealth :type "Float (double-precision)"))
  (bind _output_get (set `self.Health` (`KismetMathLibrary.FClamp` (+ (`self.Health`) value) 0.0 (`self.MaxHealth`))))
  (set `self.IsDead?` (not (> _output_get 0.0)))
  (return _output_get))