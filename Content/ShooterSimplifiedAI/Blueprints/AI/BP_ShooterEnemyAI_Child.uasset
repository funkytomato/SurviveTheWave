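; Child enemy AI Blueprint for a shooter that extends its parent with its own health and weapon tuning.
; BeginPlay sets EnemyHP after the parent call.
; WeaponSetup calls the parent, then switches on weapon type to set firing, ammo, aim and reload values, treating Pistol as a machine gun and HP Rifle as a sniper.
; Mesh, transform and sound setup nodes for each weapon are disconnected and never run.
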(event `self.ReceiveBeginPlay`
  (`parent.ReceiveBeginPlay`)
  (set `self.EnemyHP` 100.0))

(fn `UserConstructionScript`
  (`parent.UserConstructionScript`))

(fn `Weapon Setup`
  (`parent.Weapon Setup`)
  (switch `/Game/ShooterSimplifiedAI/Blueprints/AI/E_AI_WeaponType` (`self.AIWeponTypes`)
    (:`NewEnumerator0`
      ;[1 1 1] AssaultRifle
      (set `self.WeaponFireRate` 0.5)
      (set `self.WeaponDamage` 3.0)
      (bind _output_get (set `self.MaxAmmo` 10))
      (set `self.AmmoInMag` _output_get)
      (set `self.WeaponRecoil` 10.0)
      (set `self.WeaponAimTime` 0.3)
      (set `self.ReloadAnimPlayRate` 1.0)
      (set `self.WeaponReloadMontage` "/Game/ShooterSimplifiedAI/Animations/AM_Reload_Rifle_Ironsights.AM_Reload_Rifle_Ironsights"))
    (:`NewEnumerator1`
      ;[1 1 1] Machine Gun
      (set `self.WeaponFireRate` 0.2)
      (set `self.WeaponDamage` 1.0)
      (bind _output_get_2 (set `self.MaxAmmo` 15))
      (set `self.AmmoInMag` _output_get_2)
      (set `self.WeaponRecoil` 20.0)
      (set `self.WeaponAimTime` 0.5)
      (set `self.ReloadAnimPlayRate` 0.8)
      (set `self.WeaponReloadMontage` "/Game/ShooterSimplifiedAI/Animations/AM_Reload_Rifle_Ironsights.AM_Reload_Rifle_Ironsights"))
    (:`NewEnumerator2`
      ;[1 1 1] Sniper Rifle
      (set `self.WeaponFireRate` 3.0)
      (set `self.WeaponDamage` 15.0)
      (bind _output_get_3 (set `self.MaxAmmo` 1))
      (set `self.AmmoInMag` _output_get_3)
      (set `self.WeaponRecoil` 5.0)
      (set `self.WeaponAimTime` 1.0)
      (set `self.ReloadAnimPlayRate` 0.8)
      (set `self.WeaponReloadMontage` "/Game/ShooterSimplifiedAI/Animations/AM_Reload_Rifle_Ironsights.AM_Reload_Rifle_Ironsights"))))